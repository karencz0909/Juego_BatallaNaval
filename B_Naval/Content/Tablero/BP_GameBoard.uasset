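; BP_GameBoard is an actor meant to lay out a square game board of cells in its Construction Script.
; Nested loops over GridSize add a child actor component per cell and compute X/Y offsets from CellSize.
; Each offset goes to SetActorRelativeLocation with no target shown, so it moves the board itself, not the new component.
; The CellClass cast is unreachable, and the event graph is empty.
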(fn `UserConstructionScript`
  (for _index (range (`self.GridSize`))
    (for _index_2 (range (`self.GridSize`))
      (`AddComponent|NODE_AddChildActorComponent-0`)
      (`self.K2_SetActorRelativeLocation` (`KismetMathLibrary.MakeVector` (* _index (`self.CellSize`)) (* _index_2 (`self.CellSize`)))))))